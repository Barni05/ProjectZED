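; NPC AI controller that runs the NPC behavior tree and tracks perceived actors as targets.
; On BeginPlay it sets up the BB_Patrol blackboard and starts BT_NPCBehaviour.
; Perception updates write any sensed actor lacking the "Enemy" tag to the EnemyName blackboard key.
; A failed sense of any actor clears that key, regardless of its tag.
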(event OnTargetPerceptionUpdated(AIPerception)
  (params (Actor :type Actor%20Object%20Reference) (Stimulus :type AI%20Stimulus%20Structure))
  (if (.bSuccessfullySensed (Utilities|Struct|BreakAIStimulus Stimulus))
    (if (not (Actor|ActorHasTag Actor "Enemy"))
      (AI|Components|Blackboard|SetValueasObject (Variables|Default|GetBlackboardComponent) (Variables|Default|GetEnemyName) Actor))
    (else
      (AI|Components|Blackboard|ClearValue (Variables|Default|GetBlackboardComponent) (Variables|Default|GetEnemyName)))))

(event EventBeginPlay
  (bind _blackboardcomponent (Class|AIController|UseBlackboard "/Game/Character/AI/BB_Patrol.BB_Patrol"))
  (Variables|Default|SetBlackboardComponent _blackboardcomponent)
  (AI|RunBehaviorTree "/Game/Character/AI/BT_NPCBehaviour.BT_NPCBehaviour"))

(event EventTick
  (params (DeltaSeconds :type Float%20%28single-precision%29)))

(fn ConstructionScript)